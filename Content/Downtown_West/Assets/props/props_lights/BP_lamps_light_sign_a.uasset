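; A Downtown West lamp prop that pairs a static mesh with a spot light and can be set lit or unlit.
; The construction script uses LightOn to swap the mesh's emissive slot between on and off materials.
; When on, LightColor drives both the emissive parameter and the spot light, and LightIntensity sets brightness.
; When off, the spot light's attenuation radius drops to zero; the event graph has no runtime logic.
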(event EventBeginPlay)

(event Collision|EventActorBeginOverlap
  (params (OtherActor :type Actor%20Object%20Reference)))

(event EventTick
  (params (DeltaSeconds :type Float%20%28single-precision%29)))

(fn ConstructionScript
  (bind _spotlight (Variables|Default|GetSpotLight))
  (bind _sm_lamps_tree_light (Variables|Default|GetSM_lamps_tree_light))
  (bind _light_color (Variables|Default|GetLight_Color))
  (if (Variables|Default|GetLight_On)
    (Rendering|Material|SetMaterial _sm_lamps_tree_light 1 "/Game/Downtown_West/Assets/props/props_light_post/MI_Light_On.MI_Light_On")
    (Rendering|Material|SetVectorParameterValueonMaterials _sm_lamps_tree_light "Emissive_Color" _light_color)
    (Rendering|Components|Light|SetLightColor _spotlight (Math|Conversions|ToLinearColor(Vector) _light_color) true)
    (Rendering|Components|Light|SetIntensity _spotlight (Variables|Default|GetLight_Intensity))
    (else
      (Rendering|Material|SetMaterial _sm_lamps_tree_light 1 "/Game/Downtown_West/Assets/props/props_light_post/MI_Light_Off.MI_Light_Off")
      (Rendering|Lighting|SetAttenuationRadius _spotlight 0.0))))